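; Dimension-boundary plane actor that publishes its position and up vector to a material parameter collection, apparently for a dimension-switch effect.
; Construction, BeginPlay and Tick write those parameters; after a short delay, it binds the player's activate/deactivate events, which only print.
; Timer-style events step the plane between height limits, but their timer setup and the interface-based switching of tagged "Dimension" actors are disconnected, leaving MoveUp, MoveDown and SwitchDimension empty.
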(event `self.ReceiveTick`
  (params (DeltaSeconds :type "Float (single-precision)"))
  (bind _plane (`self.Plane`))
  (`KismetMaterialLibrary.SetVectorParameterValue` "/Game/Systems/DimensionSystem/PC_Advanced_Data_Dimension.PC_Advanced_Data_Dimension" "Pos" (`KismetMathLibrary.Conv_VectorToLinearColor` (`SceneComponent.K2_GetComponentLocation` _plane)) :!label _label)
  (`KismetMaterialLibrary.SetVectorParameterValue` "/Game/Systems/DimensionSystem/PC_Advanced_Data_Dimension.PC_Advanced_Data_Dimension" "Direction" (`KismetMathLibrary.Conv_VectorToLinearColor` (`SceneComponent.GetUpVector` _plane)))
  (`KismetSystemLibrary.Delay` 0.1)
  (add `/Game/Characters/Player/BP_Player.ActivateDimension` (`self.Player`) (delegate `Activate`))
  (add `/Game/Characters/Player/BP_Player.DeactivateDimension` (`self.Player`) (delegate `Deactivate`)))

(event `self.ReceiveBeginPlay`
  (`|ExecutionSequence`
    (:`then_0`
      (goto _label))
    (:`then_1`
      (bind _returnvalue (`GameplayStatics.GetActorOfClass` "/Game/Characters/Player/BP_Player.BP_Player_C"))
      (set `self.Player` _returnvalue))))

(event `UpdatePos`
  (bind _plane (`self.Plane`))
  (`KismetMaterialLibrary.SetVectorParameterValue` "/Game/Systems/DimensionSystem/PC_Advanced_Data_Dimension.PC_Advanced_Data_Dimension" "Pos" (`KismetMathLibrary.Conv_VectorToLinearColor` (`SceneComponent.K2_GetComponentLocation` _plane)))
  (`KismetMaterialLibrary.SetVectorParameterValue` "/Game/Systems/DimensionSystem/PC_Advanced_Data_Dimension.PC_Advanced_Data_Dimension" "Direction" (`KismetMathLibrary.Conv_VectorToLinearColor` (`SceneComponent.GetUpVector` _plane))))

(event `Activate`
  (`KismetSystemLibrary.PrintString` "Activate"))

(event `Deactivate`
  (`KismetSystemLibrary.PrintString` "Deactivate"))

(event `Move Up`)

(event `UpUntilEnd`
  (bind _plane (`self.Plane`))
  (bind (_returnvalue_x _returnvalue_y _returnvalue_z) (`KismetMathLibrary.BreakVector` (`SceneComponent.K2_GetComponentLocation` _plane)))
  (if (< _returnvalue_z 800.0)
    (`SceneComponent.K2_SetWorldLocation` _plane (+ (`SceneComponent.K2_GetComponentLocation` _plane) (0.0 0.0 5.0)) false false)
    (`self.UpdatePos`)
    (else
      (`KismetSystemLibrary.PrintString` "Reached Top")
      (`self.ClearTimers`))))

(event `Move Down`)

(event `DownUntilEnd`
  (bind _plane (`self.Plane`))
  (bind (_returnvalue_x _returnvalue_y _returnvalue_z) (`KismetMathLibrary.BreakVector` (`SceneComponent.K2_GetComponentLocation` _plane)))
  (if (> _returnvalue_z -200.0)
    (`SceneComponent.K2_SetWorldLocation` _plane (+ (`SceneComponent.K2_GetComponentLocation` _plane) (0.0 -0.0 -5.0)) false false)
    (`self.UpdatePos`)
    (else
      (`KismetSystemLibrary.PrintString` "Reached Bottom")
      (`self.ClearTimers`)
      (`self.Switch Dimension`))))

(event `Switch Dimension`)

(fn `ClearTimers`
  (`KismetSystemLibrary.K2_ClearAndInvalidateTimerHandle` (`self.UpTimer`))
  (`KismetSystemLibrary.K2_ClearAndInvalidateTimerHandle` (`self.DownTimer`)))

(fn `UserConstructionScript`
  (bind _plane (`self.Plane`))
  (`|ExecutionSequence`
    (:`then_0`
      (`KismetMaterialLibrary.SetVectorParameterValue` "/Game/Systems/DimensionSystem/PC_Advanced_Data_Dimension.PC_Advanced_Data_Dimension" "Pos" (`KismetMathLibrary.Conv_VectorToLinearColor` (`SceneComponent.K2_GetComponentLocation` _plane)))
      (`KismetMaterialLibrary.SetVectorParameterValue` "/Game/Systems/DimensionSystem/PC_Advanced_Data_Dimension.PC_Advanced_Data_Dimension" "Direction" (`KismetMathLibrary.Conv_VectorToLinearColor` (`SceneComponent.GetUpVector` _plane))))
    (:`then_1`
      (bind _outactors (`GameplayStatics.GetAllActorsWithTag` "Dimension"))
      (set `self.Dimensions` _outactors))))