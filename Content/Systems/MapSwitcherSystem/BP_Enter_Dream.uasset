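; BP_Enter_Dream is a map-switch actor that sends the player into the dream level selected by its DreamName enum.
; When a valid BP_Player overlaps it, it saves the player and then opens that level.
; The enum's string form doubles as the level name and as the label text, which the construction script writes to TextDreamName.
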(event `self.ReceiveBeginPlay`)

(event `self.ReceiveActorBeginOverlap`
  (params (OtherActor :type "Actor Object Reference"))
  (bind _ascharacter (cast `Character` OtherActor))
  (`/Engine/EditorBlueprintResources/StandardMacros.IsValid` _ascharacter
    (:`Is Valid`
      (bind _asbp_player (cast `/Game/Characters/Player/BP_Player` _ascharacter))
      (`/Game/Characters/Player/BP_Player.SavePlayer` _asbp_player)
      (`GameplayStatics.OpenLevel` (`KismetStringLibrary.Conv_StringToName` (`|GetEnumeratorNameAsString` (`self.DreamName`)))))))

(fn `UserConstructionScript`
  (`TextRenderComponent.K2_SetText` (`self.Text_DreamName`) (`KismetTextLibrary.Conv_StringToText` (`|GetEnumeratorNameAsString` (`self.DreamName`)))))