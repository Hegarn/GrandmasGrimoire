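; Game instance that owns the game's save data, held as a BP_GG_SaveGame object and loaded asynchronously on Init.
; Loading reads the named slot or creates a fresh save object if none exists; only a successful async load calls CallOnGameLoaded.
; SavePlayer writes player data into that object and saves it sync or async.
; GetGameData exposes the object, and ResetGameData replaces it in memory without saving.
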(event `self.ReceiveInit`
  (`KismetSystemLibrary.PrintString` "Trying to load game")
  (`self.LoadGameData` true))

(event `/Game/Systems/SaveSystem/BPI_GG_SaveGame.LoadGameData`
  (params (Async :type Boolean))
  (bind _slotname (`self.SlotName`))
  (bind _slotname_2 (`self.SlotName`))
  ;[1 1 1] LoadGame
  (bind _returnvalue (`GameplayStatics.DoesSaveGameExist` (`self.SlotName`)))
  (if _returnvalue
    (if Async
      (`KismetSystemLibrary.PrintString` (`KismetStringLibrary.Concat_StrStr` "Load game in slot: " _slotname_2))
      (bind _savegame (`AsyncActionHandleSaveGame.AsyncLoadGameFromSlot` _slotname_2)
        (:`Completed`
          (bind _asbp_gg_save_game (cast `/Game/Systems/SaveSystem/BP_GG_SaveGame` _savegame)
            (:`then`
              (set `self.SavedData` _asbp_gg_save_game)
              (`self.OnGameLoaded`))
            (:`CastFailed`
              (`KismetSystemLibrary.PrintString` "Failed to load SaveGame" :!label _label)))))
      (else
        (`KismetSystemLibrary.PrintString` (`KismetStringLibrary.Concat_StrStr` "Load game in slot: " _slotname))
        (bind _returnvalue_2 (`GameplayStatics.LoadGameFromSlot` _slotname))
        (bind _asbp_gg_save_game_2 (cast `/Game/Systems/SaveSystem/BP_GG_SaveGame` _returnvalue_2)
          (:`then`
            (set `self.SavedData` _asbp_gg_save_game_2))
          (:`CastFailed`
            (goto _label)))))
    (else
      (bind _returnvalue_3 (`GameplayStatics.CreateSaveGameObject` "/Game/Systems/SaveSystem/BP_GG_SaveGame.BP_GG_SaveGame_C"))
      (set `self.SavedData` _returnvalue_3))))

(event `/Game/Systems/SaveSystem/BPI_GG_SaveGame.SaveGameData`
  (params (Async :type Boolean))
  ;[1 1 1] SaveGame
  (if Async
    (`AsyncActionHandleSaveGame.AsyncSaveGameToSlot` (`self.SavedData`) (`self.SlotName`))
    (else
      (`KismetSystemLibrary.PrintString` (`KismetStringLibrary.Concat_StrStr` "Save game to slot: " (`self.SlotName`)))
      (`GameplayStatics.SaveGameToSlot` (`self.SavedData`) (`self.SlotName`)))))

(event `/Game/Systems/SaveSystem/BPI_GG_SaveGame.SavePlayer`
  (params (PlayerSaveData :type "/Game/Systems/SaveSystem/S_PlayerSave Structure") (Async :type Boolean))
  (set `/Game/Systems/SaveSystem/BP_GG_SaveGame.PlayerSave` PlayerSaveData (`self.SavedData`))
  (`self.SaveGameData` Async))

(event `/Game/Systems/SaveSystem/BPI_GG_SaveGame.ResetGameData`
  (bind _returnvalue (`GameplayStatics.CreateSaveGameObject` "/Game/Systems/SaveSystem/BP_GG_SaveGame.BP_GG_SaveGame_C"))
  (set `self.SavedData` _returnvalue))

(fn `GetGameData`
  (returns (SaveGameData :type "/Game/Systems/SaveSystem/BP_GG_SaveGame Object Reference"))
  (return (`self.SavedData`)))