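; Actor component that shows or hides its owning BP_Maplayer_Base map layer according to the active dimension.
; It binds to the player's activate and deactivate dimension events, which switch between dimensions 2 and 1, with DoOnce gates and delays throttling repeats and postponing deactivation.
; Layers matching the active dimension, or set to dimension 0, stay visible with collision.
; Other layers are hidden with collision disabled.
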(event `ActivateDimension`
  (`/Engine/EditorBlueprintResources/StandardMacros.DoOnce` false :!label _label
    (:`Completed`
      (`/Game/Systems/MapSwitcherSystem/BPI_DimensionSwitcher.ChangeActiveDimension` 2.0)
      (`KismetSystemLibrary.Delay` 1.0)
      (goto _label :!via `Reset`))))

(event `DeactivateDimension`
  (`/Engine/EditorBlueprintResources/StandardMacros.DoOnce` false :!label _label_2
    (:`Completed`
      (`KismetSystemLibrary.Delay` 2.0)
      (`/Game/Systems/MapSwitcherSystem/BPI_DimensionSwitcher.ChangeActiveDimension` 1.0)
      (goto _label_2 :!via `Reset`))))

(event `self.ReceiveBeginPlay`
  (`|ExecutionSequence`
    (:`then_0`
      (bind _returnvalue (`GameplayStatics.GetActorOfClass` "/Game/Characters/Player/BP_Player.BP_Player_C"))
      (set `self.Player` _returnvalue))
    (:`then_1`
      (`KismetSystemLibrary.Delay` 0.1)
      (add `/Game/Characters/Player/BP_Player.ActivateDimension` (`self.Player`) (delegate `ActivateDimension`))
      (add `/Game/Characters/Player/BP_Player.DeactivateDimension` (`self.Player`) (delegate `DeactivateDimension`)))
    (:`then_2`
      (bind _astest_actor (cast `/Game/Maps/Layers/BP_Maplayer_Base` (`self.GetOwner`)))
      (set `self.Owner` _astest_actor)
      (bind _output_get (set `self.OwningMesh` (`/Game/Maps/Layers/BP_Maplayer_Base.StaticMesh` _astest_actor)))
      (`MeshComponent.SetOverlayMaterial` _output_get (`MeshComponent.GetOverlayMaterial` _output_get))
      (bind _returnvalue_2 (`PrimitiveComponent.GetMaterial` _output_get 0))
      (`PrimitiveComponent.SetMaterial` _output_get 0 _returnvalue_2)
      (`PrimitiveComponent.SetMaterial` _output_get 1 _returnvalue_2))))

(event `/Game/Systems/MapSwitcherSystem/BPI_DimensionSwitcher.SetMaterial`
  (bind _owningmesh (`self.OwningMesh`))
  (`MeshComponent.SetOverlayMaterial` _owningmesh (`PrimitiveComponent.GetMaterial` _owningmesh 0)))

(event `/Game/Systems/MapSwitcherSystem/BPI_DimensionSwitcher.ChangeActiveDimension`
  (params (ActiveDimension :type "Float (double-precision)"))
  (bind _dimension (`self.Dimension`))
  (if (== ActiveDimension _dimension)
    (`self.ShowDimension` self :!label _label_3)
    (elif (== _dimension 0.0)
      (goto _label_3)
      (else
        (`self.HideDimension` self)))))

(event `/Game/Systems/MapSwitcherSystem/BPI_DimensionSwitcher.SetDimension`
  (params (Dimension :type "Float (double-precision)"))
  (set `self.Dimension` Dimension))

(fn `GetDimension`
  (returns (Dimension :type "Float (double-precision)"))
  (return (`self.Dimension`)))

(fn `HideDimension`
  (`Actor.SetActorHiddenInGame` (`self.Owner`) true)
  (`PrimitiveComponent.SetCollisionEnabled` (`self.OwningMesh`) "NoCollision"))

(fn `ShowDimension`
  (bind _owner (`self.Owner`))
  (`Actor.SetActorHiddenInGame` _owner false)
  (`SceneComponent.SetVisibility` (`Actor.RootComponent` _owner) true true)
  (`PrimitiveComponent.SetCollisionEnabled` (`self.OwningMesh`) "QueryAndPhysics"))