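; Base actor for a map layer that belongs to a numbered dimension and appears or disappears as the active dimension changes.
; ChangeActiveDimension shows the layer when dimensions match or its own is 0, otherwise hides it, toggling visibility and mesh collision.
; Construction applies the layer material to two mesh slots and the overlay, then evaluates visibility against active dimension 0.
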(event `/Game/Systems/MapSwitcherSystem/BPI_DimensionSwitcher.SetMaterial`
  (`MeshComponent.SetOverlayMaterial` (`self.StaticMesh`) (`self.LayerMaterial`)))

(event `/Game/Systems/MapSwitcherSystem/BPI_DimensionSwitcher.ChangeActiveDimension`
  (params (ActiveDimension :type "Float (double-precision)"))
  (bind _dimension (`self.Dimension`))
  (if (== ActiveDimension _dimension)
    (`self.ShowDimension` self :!label _label)
    (elif (== _dimension 0.0)
      (goto _label)
      (else
        (`self.HideDimension` self)))))

(event `/Game/Systems/MapSwitcherSystem/BPI_DimensionSwitcher.SetDimension`
  (params (Dimension :type "Float (double-precision)"))
  (set `self.Dimension` Dimension))

(fn `GetDimension`
  (returns (Dimension :type "Float (double-precision)"))
  (return (`self.Dimension`)))

(fn `HideDimension`
  (`self.SetActorHiddenInGame` self true)
  (`PrimitiveComponent.SetCollisionEnabled` (`self.StaticMesh`) "NoCollision"))

(fn `ShowDimension`
  (`self.SetActorHiddenInGame` self false)
  (`SceneComponent.SetVisibility` (`self.DefaultSceneRoot`) true true)
  (`PrimitiveComponent.SetCollisionEnabled` (`self.StaticMesh`) "QueryAndPhysics"))

(fn `UserConstructionScript`
  (bind _staticmesh (`self.StaticMesh`))
  (bind _layermaterial (`self.LayerMaterial`))
  (`MeshComponent.SetOverlayMaterial` _staticmesh _layermaterial)
  (`PrimitiveComponent.SetMaterial` _staticmesh 0 _layermaterial)
  (`PrimitiveComponent.SetMaterial` _staticmesh 1 _layermaterial)
  (`self.ChangeActiveDimension` self 0.0))