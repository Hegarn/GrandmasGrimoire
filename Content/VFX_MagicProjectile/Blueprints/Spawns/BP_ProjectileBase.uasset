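; BP_ProjectileBase is a projectile actor that plays a trail effect in flight and an impact effect on hit.
; On begin play it attaches the pooled ProjectileVFX system to its Scene component and returns it to the pool when destroyed.
; When the Sphere collision hits something, it spawns ImpactVFX at the impact point, oriented along the surface normal, then destroys itself.
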(event `self.ReceiveBeginPlay`
  (bind _returnvalue (`NiagaraFunctionLibrary.SpawnSystemAttached` (`self.ProjectileVFX`) (`self.Scene`) "None" (0.0 0.0 0.0) (struct) "SnapToTarget" true true "ManualRelease")))

(event `self.ReceiveDestroyed`
  (`FXSystemComponent.ReleaseToPool` (stale `self.ReceiveBeginPlay` _returnvalue)))

(event `self.Sphere.OnComponentHit`
  (params (HitComponent :type "PrimitiveComponent Object Reference") (OtherActor :type "Actor Object Reference") (OtherComp :type "PrimitiveComponent Object Reference") (NormalImpulse :type "Vector Structure") (Hit :type "HitResult Structure (by ref)"))
  (bind (_bblockinghit _binitialoverlap _time _distance _location _impactpoint _normal _impactnormal) (`GameplayStatics.BreakHitResult` Hit))
  (`NiagaraFunctionLibrary.SpawnSystemAtLocation` (`self.ImpactVFX`) _impactpoint (`KismetMathLibrary.MakeRotFromX` _impactnormal) (1.0 1.0 1.0) true true "AutoRelease")
  (`self.K2_DestroyActor`))

(fn `UserConstructionScript`)