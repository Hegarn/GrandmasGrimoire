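; BP_ProjectileSpawner is a spawner actor that repeatedly fires a magic projectile with an accompanying cast effect.
; On BeginPlay it starts a looping timer at the Frequency interval and also spawns once immediately.
; Each spawn creates the Projectiles class and the CastsToSpawn particle system at the Arrow component's location, using the actor's rotation.
; Projectiles spawn regardless of collision, and the effect uses auto-release pooling.
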(event `self.ReceiveBeginPlay`
  (`KismetSystemLibrary.K2_SetTimerDelegate` (delegate `Spawn`) (`self.Frequency`) true)
  (`self.Spawn`))

(event `Spawn`
  (`|SpawnActorFromClass` (`self.Projectiles`) (`KismetMathLibrary.MakeTransform` (`SceneComponent.K2_GetComponentLocation` (`self.Arrow`)) (`self.K2_GetActorRotation`)) "AlwaysSpawn" "OverrideRootScale" null null)
  (`NiagaraFunctionLibrary.SpawnSystemAtLocation` (`self.CastsToSpawn`) (`SceneComponent.K2_GetComponentLocation` (`self.Arrow`)) (`self.K2_GetActorRotation`) (1.0 1.0 1.0) true true "AutoRelease"))

(fn `UserConstructionScript`)