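; BP_DistanceMessure is a debug floor-tile marker that shows a distance label and reports it when the player hits it.
; The construction script writes the Textinfo value to four text render components.
; Hits on the floor mesh from BP_Player print that value with a "Distance:" prefix, throttled by a DoOnce that resets after a short delay.
; The distance is not calculated here, only displayed from Textinfo.
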(event `self.SM_Bld_Floor_1x1_01.OnComponentHit`
  (params (HitComponent :type "PrimitiveComponent Object Reference") (OtherActor :type "Actor Object Reference") (OtherComp :type "PrimitiveComponent Object Reference") (NormalImpulse :type "Vector Structure") (Hit :type "HitResult Structure (by ref)"))
  (bind _asbp_player (cast `/Game/Characters/Player/BP_Player` OtherActor))
  (`/Engine/EditorBlueprintResources/StandardMacros.IsValid` _asbp_player
    (:`Is Valid`
      (`/Engine/EditorBlueprintResources/StandardMacros.DoOnce` false :!label _label
        (:`Completed`
          (`KismetSystemLibrary.PrintString` (`KismetStringLibrary.Concat_StrStr` "Distance: " (`KismetTextLibrary.Conv_TextToString` (`self.Textinfo`))))
          (`KismetSystemLibrary.Delay` 0.2)
          (goto _label :!via `Reset`))))))

(fn `UserConstructionScript`
  (`TextRenderComponent.K2_SetText` (`self.TextRender`) (`self.Textinfo`))
  (`TextRenderComponent.K2_SetText` (`self.TextRender3`) (`self.Textinfo`))
  (`TextRenderComponent.K2_SetText` (`self.TextRender1`) (`self.Textinfo`))
  (`TextRenderComponent.K2_SetText` (`self.TextRender2`) (`self.Textinfo`)))